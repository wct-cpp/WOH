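; BP_BearDoll is a bear doll NPC that opens a tutorial and updates the quest display after its conversation closes.
; It builds an "E" indicator widget, then toggles it and the mesh's custom depth as interactability changes, animating the prompt when shown.
; When a char instigator closes the conversation, it fades in a Tutorial widget and sets the text on the first Quest widget found.
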(event `self.ReceiveBeginPlay`)

(event `self.ReceiveTick`
  (params (DeltaSeconds :type "Float (single-precision)")))

(event `InteractInterface.InitWidget`
  (bind _returnvalue (`|CreateWidget` "/Game/W_Indicator.W_Indicator_C" null "E"))
  (`Widget.SetVisibility` _returnvalue "Collapsed")
  (`WidgetComponent.SetWidget` (`self.Widget`) _returnvalue))

(event `InteractInterface.SetInteractableState`
  (params (bCanShowInteract :type Boolean))
  (if bCanShowInteract
    (`Widget.SetVisibility` (stale `InteractInterface.InitWidget` _returnvalue) "Visible")
    (`/Game/W_Indicator.PlayAnim` (stale `InteractInterface.InitWidget` _returnvalue))
    (`PrimitiveComponent.SetRenderCustomDepth` (`self.StaticMesh`) bCanShowInteract)
    (else
      (`Widget.SetVisibility` (stale `InteractInterface.InitWidget` _returnvalue) "Collapsed")
      (`PrimitiveComponent.SetRenderCustomDepth` (`self.StaticMesh`) bCanShowInteract))))

(event `self.AfterConversationClosed`
  (params (InstigateActor :type "Actor Object Reference"))
  (cast `/Game/Player/char` InstigateActor)
  (bind _returnvalue (`|CreateWidget` "/Game/Tutorial.Tutorial_C" (`GameplayStatics.GetPlayerController` 0)))
  (`UserWidget.AddToViewport` _returnvalue 0)
  (`/Game/Tutorial.PlayFadeInAnim` _returnvalue)
  (bind _foundwidgets (`WidgetBlueprintLibrary.GetAllWidgetsOfClass` "/Game/Quest.Quest_C"))
  (`/Game/Quest.Set Text` (`|GetArrayItem` _foundwidgets) 1))

(fn `UserConstructionScript`)