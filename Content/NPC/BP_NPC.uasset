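; BP_NPC is an interactable NPC that walks to a Kitchen-tagged target point after a conversation closes.
; InitWidget creates an "E" indicator, which SetInteractableState shows or hides along with the mesh's custom-depth rendering.
; World-space WidgetComp is styled at BeginPlay and yawed toward the player camera each Tick.
; AI MoveTo drives the walk flag and, on arrival, updates the quest widget and blocks repeat moves.
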(event `self.ReceiveBeginPlay`
  (bind _widgetcomp (`self.WidgetComp`))
  (bind _widgetcomp_2 (`self.WidgetComp`))
  (bind (_relativelocation_x _relativelocation_y _relativelocation_z) (`KismetMathLibrary.BreakVector` (`SceneComponent.RelativeLocation` _widgetcomp)))
  (`|ExecutionSequence`
    (:`then_0`
      (if (`|EnumEquality` (`WidgetComponent.GetWidgetSpace` (`self.WidgetComp`)) "World")
        (`PrimitiveComponent.SetCastShadow` (`self.WidgetComp`) false)
        (`SceneComponent.K2_SetRelativeLocation` _widgetcomp (`KismetMathLibrary.MakeVector` _relativelocation_x _relativelocation_y (+ _relativelocation_z 10.0)) false false)
        (`WidgetComponent.SetBackgroundColor` _widgetcomp_2 (struct :`R` 0.947917 :`G` 0.02885 :`B` 0.404838 :`A` 1.0))
        (`SceneComponent.SetRelativeScale3D` _widgetcomp_2 (0.5 0.5 0.5))))))

(event `self.ReceiveTick`
  (params (DeltaSeconds :type "Float (single-precision)"))
  (bind (_returnvalue_roll _returnvalue_pitch _returnvalue_yaw) (`KismetMathLibrary.BreakRotator` (`KismetMathLibrary.FindLookAtRotation` (`SceneComponent.K2_GetComponentLocation` (`self.WidgetComp`)) (`self.K2_GetActorLocation` (`GameplayStatics.GetPlayerCameraManager` 0)))))
  ;[1 1 1] 使状态条一直朝向玩家
  (if (`|EnumEquality` (`WidgetComponent.GetWidgetSpace` (`self.WidgetComp`)) "World")
    (`SceneComponent.K2_SetWorldRotation` (`self.WidgetComp`) (`KismetMathLibrary.MakeRotator` 0.0 0.0 _returnvalue_yaw) false false)))

(event `InteractInterface.InitWidget`
  ;[1 1 1] 直接实现该接口，因为这个NPC类在一个插件里
  (bind _returnvalue (`|CreateWidget` "/Game/W_Indicator.W_Indicator_C" null "E"))
  (`Widget.SetVisibility` _returnvalue "Collapsed")
  (`WidgetComponent.SetWidget` (`self.Widget`) _returnvalue))

(event `InteractInterface.SetInteractableState`
  (params (bCanShowInteract :type Boolean))
  (if bCanShowInteract
    (`Widget.SetVisibility` (stale `InteractInterface.InitWidget` _returnvalue) "Visible")
    (`/Game/W_Indicator.PlayAnim` (stale `InteractInterface.InitWidget` _returnvalue))
    (`PrimitiveComponent.SetRenderCustomDepth` (`self.Mesh`) bCanShowInteract)
    (else
      (`Widget.SetVisibility` (stale `InteractInterface.InitWidget` _returnvalue) "Collapsed")
      (`PrimitiveComponent.SetRenderCustomDepth` (`self.Mesh`) bCanShowInteract))))

(event `self.AfterConversationClosed`
  (params (InstigateActor :type "Actor Object Reference"))
  (if (not (`self.movetotarget`))
    (bind _outactors (`GameplayStatics.GetAllActorsOfClassWithTag` "/Script/Engine.TargetPoint" "Kitchen"))
    (bind _output (`|GetArrayItem` _outactors))
    (`|AIMoveTo` self (`self.K2_GetActorLocation` _output) _output 0.0
      (:`then`
        (set `self.isWalk` true))
      (:`OnSuccess`
        (set `self.isWalk` false)
        (set `self.movetotarget` true)
        (bind _foundwidgets (`WidgetBlueprintLibrary.GetAllWidgetsOfClass` "/Game/W_Quest.W_Quest_C"))
        (`/Game/W_Quest.Set Text` (`|GetArrayItem` _foundwidgets) 4)))))

(fn `UserConstructionScript`)