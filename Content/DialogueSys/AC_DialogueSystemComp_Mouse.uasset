(event `self.ReceiveTick`
  (params (DeltaSeconds :type "Float (single-precision)")))

(event `self.ReceiveBeginPlay`)

(fn `Dialogue`
  (`parent.Dialogue`)
  (switch `int` (`self.DialogueTreeIndex`)
    (:`0`
      (bind (_state _optionindex) (`self.AddDialogue` (`self.OwnerName`) "你肯定从未见过如此标准的十五字。你肯定从未见过如此标准的十五字。你肯定从未见过如此标准的十五字。你肯定从未见过如此标准的十五字。你肯定从未见过如此标准的十五字。你肯定从未见过如此标准的十五字。" (`|MakeArray` "想尝尝我的拳头吗！？" "杀了你。" "全都给你，不要欺负我 T_T" :!type "Text") "/Engine/VREditor/Sounds/UI/Camera_Shutter.Camera_Shutter"))
      (switch `EDialogueState` _state
        (:`PassThrough`
          (switch `int` _optionindex
            (:`0`
              (bind (_state_2 _optionindex_2) (`self.AddDialogue` (`self.OwnerName`) "Can I Have Some?" (`|MakeArray` "GiveCheese" "Keep Cheese" :!type "Text")))
              (switch `EDialogueState` _state_2
                (:`PassThrough`
                  (switch `int` _optionindex_2
                    (:`0`
                      (bind _state_3 (`self.AddDialogue` (`self.OwnerName`) "Thank you" (`|MakeArray` "Finish" :!type "Text")))
                      (switch `EDialogueState` _state_3
                        (:`PassThrough`
                          (`self.SetDialogueTreeIndex` 1)
                          (`self.CloseConversation`))))
                    (:`1`
                      (bind _state_4 (`self.AddDialogue` (`self.OwnerName`) "You bit meany" (`|MakeArray` "Finish" :!type "Text")))
                      (switch `EDialogueState` _state_4
                        (:`PassThrough`
                          (`self.RemoveDialogueProgress` 2)
                          (`self.CloseConversation`))))))))
            (:`1`
              (bind _state_5 (`self.AddDialogue` (`self.OwnerName`) "大姐我错了，求你了别鲨我 >_<" (`|MakeArray` "你叫我什么？" :!type "Text") null "/Game/NPC/Pawn/Praying__1__Anim_mixamo_com_Montage.Praying__1__Anim_mixamo_com_Montage"))
              (switch `EDialogueState` _state_5
                (:`PassThrough`
                  (`self.ClearDialogueProgress`)
                  (`self.CloseConversation`))))))))
    (:`1`
      (bind _state_6 (`self.AddDialogue` (`self.OwnerName`) (select `int` (`KismetMathLibrary.RandomIntegerInRange` 0 1) :`0` "You such a nice man" :`1` "Nomm Nomm") (`|MakeArray` "You're welcome" :!type "Text")))
      (switch `EDialogueState` _state_6
        (:`PassThrough`
          (`self.ClearDialogueProgress`)
          (`self.CloseConversation`))))))