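; Dialogue component for the bear doll, which greets Xiao An and serves as an in-game tutorial on the "heart world" mechanic.
; Overrides Dialogue, calling the parent, then runs a nested chain of AddDialogue nodes for tree index 0.
; A yes/no choice leads either to the explanation and room objectives (change clothes, collect and assemble blocks) or to an early exit.
; Both endings call RemoveDialogueProgress with different arguments, then close the conversation.
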(fn `Dialogue`
  (`parent.Dialogue`)
  (switch `int` (`self.DialogueTreeIndex`)
    (:`0`
      (bind (_state _optionindex) (`self.AddDialogue` (`self.OwnerName`) "早上好，小安。昨晚有没有做什么可爱的梦^_^" (`|MakeArray` "继续。" :!type "Text") "/Engine/VREditor/Sounds/UI/Camera_Shutter.Camera_Shutter"))
      (switch `EDialogueState` _state
        (:`PassThrough`
          (switch `int` _optionindex
            (:`0`
              (bind (_state_2 _optionindex_2) (`self.AddDialogue` (`self.OwnerName`) "我梦到我住在森林里…躺在很温暖的火炉旁边，还有很多罐甜甜的蜂蜜。真想今晚再做一次这个梦~" (`|MakeArray` "继续。" :!type "Text")))
              (switch `EDialogueState` _state_2
                (:`PassThrough`
                  (switch `int` _optionindex_2
                    (:`0`
                      (bind (_state_3 _optionindex_3) (`self.AddDialogue` (`self.OwnerName`) "不说这个了。妈妈好像在房间门口等你。" (`|MakeArray` "继续。" :!type "Text")))
                      (switch `EDialogueState` _state_3
                        (:`PassThrough`
                          (switch `int` _optionindex_3
                            (:`0`
                              (bind (_state_4 _optionindex_4) (`self.AddDialogue` (`self.OwnerName`) "但是你现在的心世界还比较小，没法走到她那里。让我想想，有什么办法可以稍微扩大心世界的范围…" (`|MakeArray` "………" :!type "Text")))
                              (switch `EDialogueState` _state_4
                                (:`PassThrough`
                                  (switch `int` _optionindex_4
                                    (:`0`
                                      (bind (_state_5 _optionindex_5) (`self.AddDialogue` (`self.OwnerName`) "你想问我什么是心世界？小安不记得的话我就再解释一遍吧。" (`|MakeArray` "好的。" "不用了。" :!type "Text")))
                                      (switch `EDialogueState` _state_5
                                        (:`PassThrough`
                                          (switch `int` _optionindex_5
                                            (:`0`
                                              (bind (_state_6 _optionindex_6) (`self.AddDialogue` (`self.OwnerName`) "心世界就是小安的心灵所能接受的世界，你可以在心世界里自由活动。拿这个房间举例的话，小安可以看到吧，妈妈站的地方的颜色跟房间里的颜色不同。" (`|MakeArray` "继续。" :!type "Text")))
                                              (switch `EDialogueState` _state_6
                                                (:`PassThrough`
                                                  (switch `int` _optionindex_6
                                                    (:`0`
                                                      (bind (_state_7 _optionindex_7) (`self.AddDialogue` (`self.OwnerName`) "这个房间就是小安现在的心世界。因为小安是来自星星的孩子，所以才会有心世界。其他人都是普普通通的小孩，所以看不到小安的心世界。虽然不能走到心世界外面去，但只要扩大心世界的范围，就能到别的地方，跟别人说话啦。" (`|MakeArray` "继续。" :!type "Text")))
                                                      (switch `EDialogueState` _state_7
                                                        (:`PassThrough`
                                                          (switch `int` _optionindex_7
                                                            (:`0`
                                                              (bind (_state_8 _optionindex_8) (`self.AddDialogue` (`self.OwnerName`) "想扩大心世界的话，一定要让自己的心灵平静下来。当小安感到害怕、烦躁、紧张的时候，就去找能让心灵平静下来的人和物品吧。" (`|MakeArray` "继续。" :!type "Text")))
                                                              (switch `EDialogueState` _state_8
                                                                (:`PassThrough`
                                                                  (switch `int` _optionindex_8
                                                                    (:`0`
                                                                      (bind (_state_9 _optionindex_9) (`self.AddDialogue` (`self.OwnerName`) "这个房间里有什么东西可以让小安的心灵安定下来呢？" (`|MakeArray` "继续。" :!type "Text")))
                                                                      (switch `EDialogueState` _state_9
                                                                        (:`PassThrough`
                                                                          (switch `int` _optionindex_9
                                                                            (:`0`
                                                                              (bind (_state_10 _optionindex_10) (`self.AddDialogue` (`self.OwnerName`) "桌上有小安昨晚还没拼完的积木。拼好积木还需要四个心形积木和一个屋顶积木。心形积木就掉在房间的地板上，把它们收集齐，然后拼到桌上的积木房子上吧。" (`|MakeArray` "继续。" :!type "Text")))
                                                                              (switch `EDialogueState` _state_10
                                                                                (:`PassThrough`
                                                                                  (switch `int` _optionindex_10
                                                                                    (:`0`
                                                                                      (bind (_state_11 _optionindex_11) (`self.AddDialogue` (`self.OwnerName`) "另外，不要忘了先去衣柜前换一下衣服哦。" (`|MakeArray` "继续。" :!type "Text")))
                                                                                      (switch `EDialogueState` _state_11
                                                                                        (:`PassThrough`
                                                                                          (switch `int` _optionindex_11
                                                                                            (:`0`
                                                                                              (bind _state_12 (`self.AddDialogue` (`self.OwnerName`) "如果有哪里不懂或忘了要做什么的话，可以随时来问我^^" (`|MakeArray` "继续。" :!type "Text")))
                                                                                              (switch `EDialogueState` _state_12
                                                                                                (:`PassThrough`
                                                                                                  (`self.RemoveDialogueProgress` 7)
                                                                                                  (`self.CloseConversation`))))))))))))))))))))))))))))
                                            (:`1`
                                              (`self.RemoveDialogueProgress` 0)
                                              (`self.CloseConversation`))))))))))))))))))))))))