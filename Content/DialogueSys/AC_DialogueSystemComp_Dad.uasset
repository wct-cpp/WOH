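; Dialogue component for the Dad NPC, who talks to Xiao An about breakfast and getting ready for school.
; It overrides the parent Dialogue function and switches on DialogueTreeIndex, chaining AddDialogue calls with single "continue" options.
; The first tree plays breakfast lines, then advances the index and closes the conversation.
; The second asks the child to find five missing notebooks, says Dad will wait at the entrance, and clears dialogue progress before closing.
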(fn `Dialogue`
  (`parent.Dialogue`)
  (switch `int` (`self.DialogueTreeIndex`)
    (:`0`
      (bind (_state _optionindex) (`self.AddDialogue` (`self.OwnerName`) "小安起来了呀。等会过来餐厅吃饭哦，吃完饭我们就去上学了。" (`|MakeArray` "继续。" :!type "Text") "/Engine/VREditor/Sounds/UI/Camera_Shutter.Camera_Shutter"))
      (switch `EDialogueState` _state
        (:`PassThrough`
          (switch `int` _optionindex
            (:`0`
              (bind (_state_2 _optionindex_2) (`self.AddDialogue` (`self.OwnerName`) "…….去学校了。" (`|MakeArray` "继续。" :!type "Text")))
              (switch `EDialogueState` _state_2
                (:`PassThrough`
                  (switch `int` _optionindex_2
                    (:`0`
                      (bind (_state_3 _optionindex_3) (`self.AddDialogue` (`self.OwnerName`) "爸爸先去厨房准备早饭哦。" (`|MakeArray` "继续。" :!type "Text")))
                      (switch `EDialogueState` _state_3
                        (:`PassThrough`
                          (switch `int` _optionindex_3
                            (:`0`
                              (`self.SetDialogueTreeIndex` 1)
                              (`self.CloseConversation`))))))))))))))
    (:`1`
      (bind _state_4 (`self.AddDialogue` (`self.OwnerName`) "小安，我们等会要去学校了。我帮你检查了书包，还缺五本笔记 \n本，小安可以找一下在哪里吗？" (`|MakeArray` "继续" :!type "Text")))
      (switch `EDialogueState` _state_4
        (:`PassThrough`
          (`self.AddDialogue` (`self.OwnerName`) "我在玄关等你哦。" (`|MakeArray` "继续" :!type "Text"))
          (`self.ClearDialogueProgress`)
          (`self.CloseConversation`))))))