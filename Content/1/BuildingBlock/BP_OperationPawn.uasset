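; BP_OperationPawn is a player pawn for selecting and manipulating the pieces of a building-block puzzle or assembly actor.
; On BeginPlay it spawns a BP_BuildingBlock and stores its four blocks in an array.
; The Zoom axis steps a clamped index through that array, highlighting the selected mesh with custom depth rendering.
; Rotation and translation axis inputs forward the selected mesh and axis value to BP_BuildingBlock's per-axis functions.
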(event `self.ReceiveBeginPlay`
  (bind _returnvalue (`|SpawnActorFromClass` "/Game/1/BuildingBlock/BP_BuildingBlock.BP_BuildingBlock_C" (`KismetMathLibrary.MakeTransform` (`self.Location`) (`self.Rotation`)) "Undefined" "OverrideRootScale" null null))
  (set `self.BP_BuildingBlock` _returnvalue)
  (`KismetArrayLibrary.Array_Add` (`self.Actors`) (`/Game/1/BuildingBlock/BP_BuildingBlock.Block1` _returnvalue))
  (`KismetArrayLibrary.Array_Add` (`self.Actors`) (`/Game/1/BuildingBlock/BP_BuildingBlock.Block2` _returnvalue))
  (`KismetArrayLibrary.Array_Add` (`self.Actors`) (`/Game/1/BuildingBlock/BP_BuildingBlock.Block3` _returnvalue))
  (`KismetArrayLibrary.Array_Add` (`self.Actors`) (`/Game/1/BuildingBlock/BP_BuildingBlock.Block4` _returnvalue))
  (`self.Select` 0.0))

(event `InputAxis|Zoom`
  (params (AxisValue :type "Float (single-precision)"))
  (`self.Select` AxisValue))

(event `InputAxis|rotateX`
  (params (AxisValue :type "Float (single-precision)"))
  (`/Game/1/BuildingBlock/BP_BuildingBlock.RotateX` (`self.BP_BuildingBlock`) (`self.SelectedMesh`) AxisValue))

(event `InputAxis|rotateY`
  (params (AxisValue :type "Float (single-precision)"))
  (`/Game/1/BuildingBlock/BP_BuildingBlock.RotateY` (`self.BP_BuildingBlock`) (`self.SelectedMesh`) AxisValue))

(event `InputAxis|rotateZ`
  (params (AxisValue :type "Float (single-precision)"))
  (`/Game/1/BuildingBlock/BP_BuildingBlock.RotateZ` (`self.BP_BuildingBlock`) (`self.SelectedMesh`) AxisValue))

(event `InputAxis|translationX`
  (params (AxisValue :type "Float (single-precision)"))
  (`/Game/1/BuildingBlock/BP_BuildingBlock.TranslationX` (`self.BP_BuildingBlock`) (`self.SelectedMesh`) AxisValue))

(event `InputAxis|translationY`
  (params (AxisValue :type "Float (single-precision)"))
  (`/Game/1/BuildingBlock/BP_BuildingBlock.TranslationY` (`self.BP_BuildingBlock`) (`self.SelectedMesh`) AxisValue))

(event `InputAxis|translationZ`
  (params (AxisValue :type "Float (single-precision)"))
  (`/Game/1/BuildingBlock/BP_BuildingBlock.TranslationZ` (`self.BP_BuildingBlock`) (`self.SelectedMesh`) AxisValue))

(fn `Select`
  (params (`Axis Value` :type "Float (double-precision)"))
  (bind _output (`|GetArrayItem` (`self.Actors`) (`self.SelectedIndex`)))
  (set `self.SelectedIndex` (`KismetMathLibrary.Clamp` (+ (`KismetMathLibrary.FTrunc` `Axis Value`) (`self.SelectedIndex`)) 0 (- (`KismetArrayLibrary.Array_Length` (`self.Actors`)) 1)))
  (`/Engine/EditorBlueprintResources/StandardMacros.IsValid` (`self.SelectedMesh`)
    (:`Is Valid`
      (`PrimitiveComponent.SetRenderCustomDepth` (`self.SelectedMesh`) false)
      (`/Engine/EditorBlueprintResources/StandardMacros.IsValid` _output
        (:`Is Valid`
          _)))
    (:`Is Not Valid`
      _))
  (bind _output_get (set `self.SelectedMesh` _output))
  (`PrimitiveComponent.SetRenderCustomDepth` _output_get true))

(fn `UserConstructionScript`)