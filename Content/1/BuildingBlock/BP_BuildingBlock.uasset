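; Building-block puzzle actor: the player moves and rotates four blocks into frame outlines, and completing it unlocks the bedroom door.
; Movement events affect only Movable blocks, while Tick checks each block against two interchangeable frames.
; Within a threshold, CheckOverlap disables input and interpolates the block into place, then locks it Static and removes it from BP_OperationPawn.
; An empty list returns control to Char and updates the quest UI.
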(event `self.ReceiveTick`
  (params (DeltaSeconds :type "Float (single-precision)"))
  (bind _returnvalue (`GameplayStatics.GetPlayerController` 0))
  (`|ExecutionSequence`
    (:`then_0`
      (`self.CheckOverlap` (`self.Block1`) (`self.BlockFrame1`))
      (`self.CheckOverlap` (`self.Block1`) (`self.BlockFrame2`))
      (`self.CheckOverlap` (`self.Block2`) (`self.BlockFrame1`))
      (`self.CheckOverlap` (`self.Block2`) (`self.BlockFrame2`))
      (`self.CheckOverlap` (`self.Block3`) (`self.BlockFrame3`))
      (`self.CheckOverlap` (`self.Block3`) (`self.BlockFrame4`))
      (`self.CheckOverlap` (`self.Block4`) (`self.BlockFrame3`))
      (`self.CheckOverlap` (`self.Block4`) (`self.BlockFrame4`)))
    (:`then_1`
      (bind _asbp_operation_pawn (cast `/Game/1/BuildingBlock/BP_OperationPawn` (`GameplayStatics.GetPlayerPawn` 0)))
      ;[1 1 1] 拼好后
      (if (== (`KismetArrayLibrary.Array_Length` (`/Game/1/BuildingBlock/BP_OperationPawn.Actors` _asbp_operation_pawn)) 0)
        (bind _returnvalue_2 (`GameplayStatics.GetActorOfClass` "/Game/Player/char.char_C"))
        (`PlayerController.SetViewTargetWithBlend` _returnvalue _returnvalue_2 1.0 "VTBlend_Linear" 0.0 false)
        (`self.SetActorHiddenInGame` _returnvalue_2 false)
        (`KismetSystemLibrary.Delay` 1.0)
        (`Controller.Possess` _returnvalue _returnvalue_2)
        (message `InteractInterface.CloseInteract` _returnvalue_2)
        (`KismetSystemLibrary.Delay` 1.0)
        (`/Game/Player/char.changeRange1` _returnvalue_2 (`self.AddRange`))
        ;[1 1 1] 门开启的声音
        (`GameplayStatics.PlaySound2D` "/Game/sound/开门音效_耳聆网__声音ID：15761_.开门音效_耳聆网__声音ID：15761_" 1.0 1.0 0.0 null null)
        (bind _outactors (`GameplayStatics.GetAllActorsOfClassWithTag` "/Game/Interactable/BP_Door.BP_Door_C" "BedroomDoor"))
        (set `/Game/Interactable/BP_Door.bIsLocked` false (`|GetArrayItem` _outactors))
        (bind _foundwidgets (`WidgetBlueprintLibrary.GetAllWidgetsOfClass` "/Game/W_Quest.W_Quest_C"))
        (`/Game/W_Quest.Set Text` (`|GetArrayItem` _foundwidgets) 3)
        (bind _foundwidgets_2 (`WidgetBlueprintLibrary.GetAllWidgetsOfClass` "/Game/1/BuildingBlock/W_BuildingBlockInstruct.W_BuildingBlockInstruct_C" false))
        (`Widget.RemoveFromParent` (`|GetArrayItem` _foundwidgets_2))))))

(event `RotateX`
  (params (Block :type "StaticMeshComponent Object Reference") (value :type "Float (double-precision)"))
  (if (`|EnumEquality` (`SceneComponent.Mobility` Block) "Movable")
    (`SceneComponent.K2_AddLocalRotation` Block (`KismetMathLibrary.MakeRotator` value) false false)))

(event `RotateY`
  (params (Block :type "StaticMeshComponent Object Reference") (value :type "Float (double-precision)"))
  (if (`|EnumEquality` (`SceneComponent.Mobility` Block) "Movable")
    (`SceneComponent.K2_AddLocalRotation` Block (`KismetMathLibrary.MakeRotator` 0.0 value) false false)))

(event `RotateZ`
  (params (Block :type "StaticMeshComponent Object Reference") (value :type "Float (double-precision)"))
  (if (`|EnumEquality` (`SceneComponent.Mobility` Block) "Movable")
    (`SceneComponent.K2_AddLocalRotation` Block (`KismetMathLibrary.MakeRotator` 0.0 0.0 value) false false)))

(event `TranslationX`
  (params (Block :type "StaticMeshComponent Object Reference") (value :type "Float (double-precision)"))
  (if (`|EnumEquality` (`SceneComponent.Mobility` Block) "Movable")
    (`SceneComponent.K2_AddRelativeLocation` Block (`KismetMathLibrary.MakeVector` value) false false)))

(event `TranslationY`
  (params (Block :type "StaticMeshComponent Object Reference") (value :type "Float (double-precision)"))
  (if (`|EnumEquality` (`SceneComponent.Mobility` Block) "Movable")
    (`SceneComponent.K2_AddRelativeLocation` Block (`KismetMathLibrary.MakeVector` 0.0 value) false false)))

(event `TranslationZ`
  (params (Block :type "StaticMeshComponent Object Reference") (value :type "Float (double-precision)"))
  (if (`|EnumEquality` (`SceneComponent.Mobility` Block) "Movable")
    (`SceneComponent.K2_AddRelativeLocation` Block (`KismetMathLibrary.MakeVector` 0.0 0.0 value) false false)))

(fn `CheckOverlap`
  (params (Block :type "StaticMeshComponent Object Reference") (BlockFrame :type "StaticMeshComponent Object Reference"))
  (bind (_relativerotation_roll _relativerotation_pitch _relativerotation_yaw) (`KismetMathLibrary.BreakRotator` (`SceneComponent.RelativeRotation` BlockFrame)))
  (bind (_relativerotation_roll_2 _relativerotation_pitch_2 _relativerotation_yaw_2) (`KismetMathLibrary.BreakRotator` (`SceneComponent.RelativeRotation` Block)))
  (if (`SceneComponent.bVisible` BlockFrame)
    (if (and (< (`KismetMathLibrary.Vector_Distance` (`SceneComponent.RelativeLocation` Block) (`SceneComponent.RelativeLocation` BlockFrame)) (`self.Threshold`)) (< (`KismetMathLibrary.Abs` (- _relativerotation_roll_2 _relativerotation_roll)) (`self.Threshold`)) (< (`KismetMathLibrary.Abs` (- _relativerotation_pitch_2 _relativerotation_pitch)) (`self.Threshold`)) (< (`KismetMathLibrary.Abs` (- _relativerotation_yaw_2 _relativerotation_yaw)) (`self.Threshold`)))
      (`self.DisableInput` (`GameplayStatics.GetPlayerPawn` 0) (`GameplayStatics.GetPlayerController` 0))
      (`SceneComponent.K2_SetRelativeLocationAndRotation` (`local.Block`) (`KismetMathLibrary.VInterpTo` (`SceneComponent.RelativeLocation` (`local.Block`)) (`SceneComponent.RelativeLocation` (`local.BlockFrame`)) 0.1 0.3) (`KismetMathLibrary.RInterpTo` (`SceneComponent.RelativeRotation` (`local.Block`)) (`SceneComponent.RelativeRotation` (`local.BlockFrame`)) 0.1 0.3) false false)
      ;[1 1 1] 重合之后
      (if (== (`SceneComponent.RelativeLocation` (`local.Block`)) (`SceneComponent.RelativeLocation` (`local.BlockFrame`)))
        (`SceneComponent.SetVisibility` (`local.BlockFrame`) false false)
        (`SceneComponent.SetMobility` (`local.Block`) "Static")
        (`PrimitiveComponent.SetRenderCustomDepth` (`local.Block`) false)
        (bind _asbp_operation_pawn (cast `/Game/1/BuildingBlock/BP_OperationPawn` (`GameplayStatics.GetPlayerPawn` 0)))
        (`KismetArrayLibrary.Array_RemoveItem` (`/Game/1/BuildingBlock/BP_OperationPawn.Actors` _asbp_operation_pawn) (`local.Block`))
        (`self.EnableInput` (`GameplayStatics.GetPlayerPawn` 0) (`GameplayStatics.GetPlayerController` 0))))))

(fn `UserConstructionScript`)