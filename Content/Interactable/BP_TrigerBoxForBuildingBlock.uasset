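; BP_TrigerBoxForBuildingBlock is an interactable trigger box that hands player control to BP_OperationPawn, presumably for a building-block activity.
; Box overlap begin and end events toggle the interactable state, showing and animating or collapsing an "E" indicator in a widget component.
; Interact hides the instigator, blends the camera to the first BP_OperationPawn found, then possesses it after a delay matching the blend.
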(event `InteractInterface.InitWidget`
  (bind _returnvalue (`|CreateWidget` "/Game/W_Indicator.W_Indicator_C" null "E"))
  (`Widget.SetVisibility` _returnvalue "Collapsed")
  (`WidgetComponent.SetWidget` (`self.Widget`) _returnvalue))

(event `InteractInterface.SetInteractableState`
  (params (bCanShowInteract :type Boolean))
  (if bCanShowInteract
    (`Widget.SetVisibility` (stale `InteractInterface.InitWidget` _returnvalue) "Visible")
    (`/Game/W_Indicator.PlayAnim` (stale `InteractInterface.InitWidget` _returnvalue))
    (else
      (`Widget.SetVisibility` (stale `InteractInterface.InitWidget` _returnvalue) "Collapsed"))))

(event `self.Box.OnComponentBeginOverlap`
  (params (OverlappedComponent :type "PrimitiveComponent Object Reference") (OtherActor :type "Actor Object Reference") (OtherComp :type "PrimitiveComponent Object Reference") (OtherBodyIndex :type Integer) (bFromSweep :type Boolean) (SweepResult :type "HitResult Structure (by ref)"))
  (message `InteractInterface.SetInteractableState` self true))

(event `InteractInterface.Interact`
  (params (InstigateActor :type "Actor Object Reference"))
  (bind _returnvalue (`GameplayStatics.GetPlayerController` 0))
  (`self.SetActorHiddenInGame` InstigateActor true)
  (bind _returnvalue_2 (`GameplayStatics.GetActorOfClass` "/Game/1/BuildingBlock/BP_OperationPawn.BP_OperationPawn_C"))
  (`PlayerController.SetViewTargetWithBlend` _returnvalue _returnvalue_2 1.0 "VTBlend_Linear" 0.0 false)
  (`KismetSystemLibrary.Delay` 1.0)
  (`Controller.Possess` _returnvalue _returnvalue_2))

(event `self.Box.OnComponentEndOverlap`
  (params (OverlappedComponent :type "PrimitiveComponent Object Reference") (OtherActor :type "Actor Object Reference") (OtherComp :type "PrimitiveComponent Object Reference") (OtherBodyIndex :type Integer))
  (message `InteractInterface.SetInteractableState` self false))

(fn `UserConstructionScript`)