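; BP_Door2 is an interactable sliding door that works only when the player is on its forward side, checked by a dot product.
; SetInteractableState shows an animated "E" prompt widget under that same check.
; Interact alternates through a FlipFlop between playing and reversing a timeline that offsets the root's relative X, with direction set by IsLeft.
; The instigator's interact message closes when the timeline finishes or the side check fails.
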(event `InteractInterface.InitWidget`
  (bind _returnvalue (`|CreateWidget` "/Game/W_Indicator.W_Indicator_C" null "E"))
  (`Widget.SetVisibility` _returnvalue "Collapsed")
  (`WidgetComponent.SetWidget` (`self.Widget`) _returnvalue))

(event `InteractInterface.SetInteractableState`
  (params (bCanShowInteract :type Boolean))
  (if (and bCanShowInteract (> (`KismetMathLibrary.Dot_VectorVector` (- (`self.K2_GetActorLocation` (`GameplayStatics.GetPlayerPawn` 0)) (`self.K2_GetActorLocation`)) (`SceneComponent.GetForwardVector` (`self.DefaultSceneRoot`))) 0.0))
    (`Widget.SetVisibility` (stale `InteractInterface.InitWidget` _returnvalue) "Visible")
    (`/Game/W_Indicator.PlayAnim` (stale `InteractInterface.InitWidget` _returnvalue))
    (else
      (`Widget.SetVisibility` (stale `InteractInterface.InitWidget` _returnvalue) "Collapsed"))))

(event `self.ReceiveBeginPlay`
  (if (`self.bIsLeft`)
    (set `self.倍率` -100.0)
    (else
      (set `self.倍率` 100.0))))

(event `InteractInterface.Interact`
  (params (InstigateActor :type "Actor Object Reference"))
  (bind (_relativelocation_x _relativelocation_y _relativelocation_z) (`KismetMathLibrary.BreakVector` (`SceneComponent.RelativeLocation` (`self.DefaultSceneRoot`))))
  (bind _relativelocation_x_2 (`KismetMathLibrary.BreakVector` (`SceneComponent.RelativeLocation` (`self.DefaultSceneRoot`))))
  (if (> (`KismetMathLibrary.Dot_VectorVector` (- (`self.K2_GetActorLocation` (`GameplayStatics.GetPlayerPawn` 0)) (`self.K2_GetActorLocation`)) (`SceneComponent.GetForwardVector` (`self.DefaultSceneRoot`))) 0.0)
    (`/Engine/EditorBlueprintResources/StandardMacros.FlipFlop`
      (:`A`
        (set `self.pre 相对位置 X` _relativelocation_x_2)
        (bind (_direction `_新建轨道_0`) (`Timeline|时间轴_0` :!via `PlayFromStart` :!label _label)
          (:`Update`
            (`SceneComponent.K2_SetRelativeLocation` (`self.DefaultSceneRoot`) (`KismetMathLibrary.MakeVector` (+ (`self.pre 相对位置 X`) (* `_新建轨道_0` (`self.倍率`))) _relativelocation_y _relativelocation_z) false false))
          (:`Finished`
            (message `InteractInterface.CloseInteract` InstigateActor))))
      (:`B`
        (goto _label :!via `ReverseFromEnd`)))
    (else
      (message `InteractInterface.CloseInteract` InstigateActor))))

(fn `UserConstructionScript`)