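; BP_BuildingBlockSolo is an interactable building-block pickup that counts toward a four-block quest.
; It shows an "E" indicator widget and custom-depth render on its mesh while interactable.
; Interact hides the mesh, increments the character's block count and closes the interact message.
; At four or more blocks it spawns BP_OperationPawn at fixed coordinates, enables the trigger box's query collision, destroys itself and updates the W_Quest text.
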(event `InteractInterface.InitWidget`
  (bind _returnvalue (`|CreateWidget` "/Game/W_Indicator.W_Indicator_C" null "E"))
  (`Widget.SetVisibility` _returnvalue "Collapsed")
  (`WidgetComponent.SetWidget` (`self.Widget`) _returnvalue))

(event `InteractInterface.SetInteractableState`
  (params (bCanShowInteract :type Boolean))
  (if bCanShowInteract
    (`Widget.SetVisibility` (stale `InteractInterface.InitWidget` _returnvalue) "Visible")
    (`/Game/W_Indicator.PlayAnim` (stale `InteractInterface.InitWidget` _returnvalue))
    (`PrimitiveComponent.SetRenderCustomDepth` (`self.StaticMesh`) bCanShowInteract)
    (else
      (`Widget.SetVisibility` (stale `InteractInterface.InitWidget` _returnvalue) "Collapsed")
      (`PrimitiveComponent.SetRenderCustomDepth` (`self.StaticMesh`) bCanShowInteract))))

(event `InteractInterface.Interact`
  (params (InstigateActor :type "Actor Object Reference"))
  (`SceneComponent.SetVisibility` (`self.StaticMesh`) false false)
  (bind _aschar (cast `/Game/Player/char` InstigateActor))
  (bind _numofbuildingblocks (`/Game/Player/char.NumOfBuildingBlocks` _aschar))
  (set `/Game/Player/char.NumOfBuildingBlocks` (+ _numofbuildingblocks 1) _aschar)
  (message `InteractInterface.CloseInteract` InstigateActor)
  (if (>= _numofbuildingblocks 4)
    (`|ExecutionSequence`
      (:`then_0`
        (`|SpawnActorFromClass` "/Game/1/BuildingBlock/BP_OperationPawn.BP_OperationPawn_C" (`KismetMathLibrary.MakeTransform` (1195.0 -869.0 164.0) (struct :`Pitch` -10.0)) "Undefined" "OverrideRootScale" null null))
      (:`then_1`
        (bind _returnvalue (`GameplayStatics.GetActorOfClass` "/Game/Interactable/BP_TrigerBoxForBuildingBlock.BP_TrigerBoxForBuildingBlock_C"))
        (`PrimitiveComponent.SetCollisionEnabled` (`/Game/Interactable/BP_TrigerBoxForBuildingBlock.Box` _returnvalue) "QueryOnly")
        (`self.K2_DestroyActor`))
      (:`then_2`
        (bind _foundwidgets (`WidgetBlueprintLibrary.GetAllWidgetsOfClass` "/Game/W_Quest.W_Quest_C"))
        (`/Game/W_Quest.Set Text` (`|GetArrayItem` _foundwidgets) 2)))))

(fn `UserConstructionScript`)