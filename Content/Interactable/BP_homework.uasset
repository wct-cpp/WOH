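; BP_homework is an interactable book pickup that counts toward a five-book quest.
; A widget component shows an animated "E" indicator and the mesh enables custom depth while interaction is available.
; Interacting hides the mesh without destroying the actor, plays a sound, increments the character's book count and closes the interact message.
; At five or more books, it updates the W_Quest widget and opens the "Untitled" level after a delay.
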(event `InteractInterface.InitWidget`
  (bind _returnvalue (`|CreateWidget` "/Game/W_Indicator.W_Indicator_C" null "E"))
  (`Widget.SetVisibility` _returnvalue "Collapsed")
  (`WidgetComponent.SetWidget` (`self.Widget`) _returnvalue))

(event `InteractInterface.SetInteractableState`
  (params (bCanShowInteract :type Boolean))
  (if bCanShowInteract
    (`Widget.SetVisibility` (stale `InteractInterface.InitWidget` _returnvalue) "Visible")
    (`/Game/W_Indicator.PlayAnim` (stale `InteractInterface.InitWidget` _returnvalue))
    (`PrimitiveComponent.SetRenderCustomDepth` (`self.StaticMesh`) bCanShowInteract)
    (else
      (`Widget.SetVisibility` (stale `InteractInterface.InitWidget` _returnvalue) "Collapsed")
      (`PrimitiveComponent.SetRenderCustomDepth` (`self.StaticMesh`) bCanShowInteract))))

(event `InteractInterface.Interact`
  (params (InstigateActor :type "Actor Object Reference"))
  (`SceneComponent.SetVisibility` (`self.StaticMesh`) false false)
  ;[1 1 1] 收书声音
  (`GameplayStatics.PlaySound2D` null 1.0 1.0 0.0 null null)
  (bind _aschar (cast `/Game/Player/char` InstigateActor))
  (bind _output_get (set `/Game/Player/char.NumOfBooks` (+ (`/Game/Player/char.NumOfBooks` _aschar) 1) _aschar))
  (message `InteractInterface.CloseInteract` InstigateActor)
  (if (>= _output_get 5)
    (`|ExecutionSequence`
      (:`then_0`
        (bind _foundwidgets (`WidgetBlueprintLibrary.GetAllWidgetsOfClass` "/Game/W_Quest.W_Quest_C"))
        (`/Game/W_Quest.Set Text` (`|GetArrayItem` _foundwidgets) 6))
      (:`then_1`
        (`KismetSystemLibrary.Delay` 2.0)
        (`GameplayStatics.OpenLevel` "Untitled")))))

(fn `UserConstructionScript`)