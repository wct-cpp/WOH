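; Interactable door that swings 90 degrees open or shut, with an "E" prompt widget that shows and animates while interaction is available.
; Interact compares the current yaw to the BeginPlay yaw to pick the swing direction, then a timeline rotates the root and closes the instigator's interact message when finished.
; A dot product tests the instigator's side, but both branches end up with the same swing direction.
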(event `self.ReceiveBeginPlay`
  (bind (_relativerotation_roll _relativerotation_pitch _relativerotation_yaw) (`KismetMathLibrary.BreakRotator` (`SceneComponent.RelativeRotation` (`self.DefaultSceneRoot`))))
  (set `self.初始 相对旋转 Z (Yaw)` _relativerotation_yaw))

(event `InteractInterface.InitWidget`
  (bind _returnvalue (`|CreateWidget` "/Game/W_Indicator.W_Indicator_C" null "E"))
  (`Widget.SetVisibility` _returnvalue "Collapsed")
  (`WidgetComponent.SetWidget` (`self.Widget`) _returnvalue))

(event `InteractInterface.SetInteractableState`
  (params (bCanShowInteract :type Boolean))
  (if bCanShowInteract
    (`Widget.SetVisibility` (stale `InteractInterface.InitWidget` _returnvalue) "Visible")
    (`/Game/W_Indicator.PlayAnim` (stale `InteractInterface.InitWidget` _returnvalue))
    (else
      (`Widget.SetVisibility` (stale `InteractInterface.InitWidget` _returnvalue) "Collapsed"))))

(event `self.ReceiveTick`
  (params (DeltaSeconds :type "Float (single-precision)")))

(event `InteractInterface.Interact`
  (params (InstigateActor :type "Actor Object Reference"))
  (bind (_relativerotation_roll _relativerotation_pitch _relativerotation_yaw) (`KismetMathLibrary.BreakRotator` (`SceneComponent.RelativeRotation` (`self.DefaultSceneRoot`))))
  (bind _output_get (set `self.pre 相对旋转 Z (Yaw)` _relativerotation_yaw))
  (if (> (`KismetMathLibrary.Dot_VectorVector` (- (`self.K2_GetActorLocation` InstigateActor) (`self.K2_GetActorLocation`)) (`SceneComponent.GetForwardVector` (`self.DefaultSceneRoot`))) 0.0)
    (set `self.倍率` -90.0)
    (bind _returnvalue (> (- _output_get (`self.初始 相对旋转 Z (Yaw)`)) 1.0))
    (if _returnvalue
      (bind (_direction `_新建轨道_0`) (`Timeline|时间轴_0` :!via `PlayFromStart` :!label _label)
        (:`Update`
          (`SceneComponent.K2_SetRelativeRotation` (`self.DefaultSceneRoot`) (`KismetMathLibrary.MakeRotator` 0.0 0.0 (+ (* `_新建轨道_0` (`self.倍率`)) (`self.pre 相对旋转 Z (Yaw)`))) false false))
        (:`Finished`
          (message `InteractInterface.CloseInteract` InstigateActor)))
      (else
        (set `self.倍率` 90.0)
        (goto _label :!via `PlayFromStart`)))
    (else
      (set `self.倍率` 90.0)
      (if _returnvalue
        (set `self.倍率` -90.0)
        (goto _label :!via `PlayFromStart`)
        (else
          (goto _label :!via `PlayFromStart`))))))

(fn `UserConstructionScript`)