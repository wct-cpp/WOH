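; Voxel terrain generator actor that builds a grid of height-scaled instances for water, beach and grass.
; GenerateGrid optionally randomizes the noise offset, clears the three instanced static meshes, then adds one instance per cell.
; Each cell's height sums mountain and boulder noise layers, clamped to a minimum, and is compared with water level and beach size to pick its mesh.
; Height is applied as instance Z scale, so each cell is a single column.
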(event `self.ReceiveBeginPlay`)

(event `ClearGrid`
  (`InstancedStaticMeshComponent.ClearInstances` (`self.ISM_Grass`))
  (`InstancedStaticMeshComponent.ClearInstances` (`self.ISM_Water`))
  (`InstancedStaticMeshComponent.ClearInstances` (`self.ISM_Beach`)))

(event `GenerateGrid`
  (bind _returnvalue (* (`KismetMathLibrary.RandomFloat`) 5000000000.0))
  (bind _returnvalue_2 (- (`KismetMathLibrary.Conv_IntToDouble` (/ (`self.xWidth`) (`self.VoxelSize`))) 0.03))
  (if (`self.RandomizeLayout`)
    (set `self.PerlinOffset` (`KismetMathLibrary.MakeVector2D` _returnvalue _returnvalue)))
  (`self.ClearGrid`)
  (for _index (range (+ (`self.YCellCount`) 1))
    (for _index_2 (range (+ (`self.XCellCount`) 1))
      (bind _celllocation (`self.CalculateCellLocation` _index_2 _index))
      (bind (_returnvalue_3 _ism) (`self.GetHeightAndType` _celllocation))
      (`InstancedStaticMeshComponent.AddInstance` _ism (`KismetMathLibrary.MakeTransform` _celllocation (struct) (`KismetMathLibrary.MakeVector` _returnvalue_2 _returnvalue_2 _returnvalue_3))))))

(fn `CalculateCellLocation`
  (params (x :type Integer) (y :type Integer))
  (returns (CellLocation :type "Vector Structure"))
  (return (+ (* (`KismetMathLibrary.MakeVector` (`KismetMathLibrary.Conv_IntToDouble` x) (`KismetMathLibrary.Conv_IntToDouble` y)) (`self.xWidth`)) (`self.K2_GetActorLocation`))))

(fn `GetHeightAndType`
  (params (InVector :type "Vector Structure"))
  (returns (ReturnValue :type "Float (double-precision)") (ISM :type "InstancedStaticMeshComponent Object Reference"))
  (locals (Z :type "Float (double-precision)"))
  (bind _waterlevel (`self.WaterLevel`))
  (bind _returnvalue (+ (`KismetMathLibrary.Conv_VectorToVector2D` InVector) (`self.PerlinOffset`)))
  (bind _returnvalue_2 (`self.GetTerrainHeight` _returnvalue (`self.MountainScale`) (`self.MountainHeight`)))
  (bind _returnvalue_3 (`self.GetTerrainHeight` _returnvalue (`self.BoulderScale`) (`self.BoulderAmplitude`)))
  (set `local.Z` (`KismetMathLibrary.FMax` (/ (+ _returnvalue_2 _returnvalue_3) (`KismetMathLibrary.Conv_IntToDouble` (`self.VoxelSize`))) 1.0))
  (if (== (`local.Z`) (`self.WaterLevel`))
    (return (`self.WaterLevel`) (`self.ISM_Water`))
    (elif (`KismetMathLibrary.InRange_FloatFloat` (`local.Z`) _waterlevel (+ _waterlevel (`self.BeachSize`)))
      (return (+ (`self.WaterLevel`) 1.0) (`self.ISM_Beach`))
      (else
        (set `local.Z` (`KismetMathLibrary.FMax` (- (`local.Z`) (`self.BeachSize`)) (+ (`self.WaterLevel`) 2.0)))
        (return (`local.Z`) (`self.ISM_Grass`))))))

(fn `UserConstructionScript`)