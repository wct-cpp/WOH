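; BP_VoxelGen_Hex is a voxel generator variant that positions cells on a flat hexagonal grid.
; The construction script derives row spacing (YWidth) and column spacing (XGap) from XWidth using hexagon proportions, then runs the parent script.
; CalculateCellLocation turns X/Y indices into positions offset from the actor's location, shifting odd columns half a cell along Y to interlock.
; The event graph holds only disabled default events.
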(fn `CalculateCellLocation`
  (params (x :type Integer) (y :type Integer))
  (returns (CellLocation :type "Vector Structure"))
  (return (+ (* (`KismetMathLibrary.MakeVector` (`KismetMathLibrary.Conv_IntToDouble` x) (+ (`KismetMathLibrary.Conv_IntToDouble` y) (`KismetMathLibrary.SelectFloat` 0.0 0.5 (== (mod x 2) 0)))) (`KismetMathLibrary.MakeVector` (`self.xGap`) (`self.yWidth`))) (`self.K2_GetActorLocation`))))

(fn `UserConstructionScript`
  (set `self.yWidth` (* (`self.xWidth`) (`KismetMathLibrary.DegCos` 30.0)))
  (set `self.xGap` (* (`self.xWidth`) 0.75))
  (`parent.UserConstructionScript`))