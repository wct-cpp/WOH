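; Hexagonal variant of a world-gen cell generator that lays out hex cells as child actors.
; The construction script derives column gap and row height from XWidth, then calls Generate, whose body is not in this file.
; CalculateCellLocation maps grid coordinates to positions relative to the actor's location, shifting odd columns half a cell.
; SpawnChildActor adds a child actor component, stores it in CellArray and sets the BP_HexCell's type.
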(fn `CalculateCellLocation`
  (params (x :type Integer) (y :type Integer))
  (returns (CellLocation :type "Vector Structure"))
  (return (+ (* (`KismetMathLibrary.MakeVector` (`KismetMathLibrary.Conv_IntToDouble` x) (+ (`KismetMathLibrary.Conv_IntToDouble` y) (`KismetMathLibrary.SelectFloat` 0.0 0.5 (== (mod x 2) 0)))) (`KismetMathLibrary.MakeVector` (`self.xGap`) (`self.yWidth`))) (`self.K2_GetActorLocation`))))

(fn `SpawnChildActor`
  (params (RelativeTransform_Location :type "Vector Structure") (RelativeTransform_Scale_X :type "Float (double-precision)") (RelativeTransform_Scale_Y :type "Float (double-precision)") (RelativeTransform_Scale_Z :type "Float (double-precision)") (Type :type Integer))
  (bind _returnvalue (`AddComponent|NODE_AddChildActorComponent-1` :`RelativeTransform` (`KismetMathLibrary.MakeTransform` RelativeTransform_Location (struct) (`KismetMathLibrary.MakeVector` RelativeTransform_Scale_X RelativeTransform_Scale_Y RelativeTransform_Scale_Z))))
  (`KismetArrayLibrary.Array_Add` (`self.CellArray`) _returnvalue)
  (bind _asbp_hex_cell (cast `/Game/WorldGen/BP_HexCell` (`ChildActorComponent.ChildActor` _returnvalue)))
  (`/Game/WorldGen/BP_HexCell.SetType` _asbp_hex_cell Type)
  (return))

(fn `UserConstructionScript`
  (set `self.yWidth` (* (`self.xWidth`) (`KismetMathLibrary.DegCos` 30.0)))
  (set `self.xGap` (* (`self.xWidth`) 0.75))
  (`parent.UserConstructionScript`)
  (`self.Generate`))