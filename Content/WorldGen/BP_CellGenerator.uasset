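; BP_CellGenerator builds a grid terrain of BP_Cell child actors, with each cell's height set through its Z scale.
; Generate optionally randomizes the noise offset, destroys previous cell components, then spawns one cell per grid coordinate.
; Each height sums mountain and boulder Perlin noise layers, clamped to a minimum.
; Height exactly at WaterLevel gives water, the BeachSize band above gives beach, and all others become raised land.
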(event `Clear`
  (for _array_element (`self.CellArray`)
    (`ActorComponent.K2_DestroyComponent` _array_element)))

(event `Generate`
  (bind _returnvalue (* (`KismetMathLibrary.RandomFloat`) 5000000000.0))
  (bind _returnvalue_2 (- (`KismetMathLibrary.Conv_IntToDouble` (/ (`self.xWidth`) (`self.CellSize`))) 0.03))
  (if (`self.RandomizeLayout`)
    (set `self.PerlinOffset` (`KismetMathLibrary.MakeVector2D` _returnvalue _returnvalue)))
  (`self.Clear`)
  (for _index (range (`self.YCellCount`))
    (for _index_2 (range (`self.XCellCount`))
      (bind _celllocation (`self.CalculateCellLocation` _index_2 _index))
      (bind (_scale_z _type) (`self.SetHeightAndType` _celllocation))
      (`self.SpawnChildActor` _celllocation _returnvalue_2 _returnvalue_2 _scale_z _type))))

(fn `CalculateCellLocation`
  (params (x :type Integer) (y :type Integer))
  (returns (CellLocation :type "Vector Structure"))
  (return (+ (* (`KismetMathLibrary.MakeVector` (`KismetMathLibrary.Conv_IntToDouble` x) (`KismetMathLibrary.Conv_IntToDouble` y)) (`self.xWidth`)) (`self.K2_GetActorLocation`))))

(fn `SetHeightAndType`
  (params (CellLocation :type "Vector Structure"))
  (returns (`Scale Z` :type "Float (double-precision)") (Type :type Integer))
  (locals (Z :type "Float (double-precision)"))
  (bind _waterlevel (`self.WaterLevel`))
  (bind _returnvalue (+ (`KismetMathLibrary.Conv_VectorToVector2D` CellLocation) (`self.PerlinOffset`)))
  (bind _returnvalue_2 (`self.GetTerrainHeight` _returnvalue (`self.MountainScale`) (`self.MountainHeight`)))
  (bind _returnvalue_3 (`self.GetTerrainHeight` _returnvalue (`self.BoulderScale`) (`self.BoulderAmplitude`)))
  (set `local.Z` (`KismetMathLibrary.FMax` (/ (+ _returnvalue_2 _returnvalue_3) (`KismetMathLibrary.Conv_IntToDouble` (`self.CellSize`))) 1.0))
  (if (== (`local.Z`) (`self.WaterLevel`))
    (return (`self.WaterLevel`) 1)
    (elif (`KismetMathLibrary.InRange_FloatFloat` (`local.Z`) _waterlevel (+ _waterlevel (`self.BeachSize`)))
      (return (+ (`self.WaterLevel`) 1.0) 2)
      (else
        (set `local.Z` (`KismetMathLibrary.FMax` (- (`local.Z`) (`self.BeachSize`)) (+ (`self.WaterLevel`) 2.0)))
        (return (`local.Z`) 0)))))

(fn `SpawnChildActor`
  (params (RelativeTransform_Location :type "Vector Structure") (RelativeTransform_Scale_X :type "Float (double-precision)") (RelativeTransform_Scale_Y :type "Float (double-precision)") (RelativeTransform_Scale_Z :type "Float (double-precision)") (Type :type Integer))
  (bind _returnvalue (`AddComponent|NODE_AddChildActorComponent-3` :`RelativeTransform` (`KismetMathLibrary.MakeTransform` RelativeTransform_Location (struct) (`KismetMathLibrary.MakeVector` RelativeTransform_Scale_X RelativeTransform_Scale_Y RelativeTransform_Scale_Z))))
  (`KismetArrayLibrary.Array_Add` (`self.CellArray`) _returnvalue)
  (bind _asbp_cell (cast `/Game/WorldGen/BP_Cell` (`ChildActorComponent.ChildActor` _returnvalue)))
  (`/Game/WorldGen/BP_Cell.SetType` _asbp_cell Type)
  (return))

(fn `UserConstructionScript`)